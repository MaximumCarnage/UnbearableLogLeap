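; HUD Blueprint that adds the HUDWidget to the viewport and draws the win or lose screen for a level.
; A gate toggled by the ShowText event controls per-frame DrawHUD text, choosing win or restart prompts from the Win value of the WinLoss event.
; While showing, it also writes WinLoss and CanRestart to the first LevelDB actor, found at BeginPlay.
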(event Collision|EventActorBeginOverlap
  (params (OtherActor :type Actor%20Object%20Reference)))

(event EventShowText
  (params (ShowText? :type Boolean))
  (if ShowText?
    (Utilities|FlowControl|Gate true) ; enters at Open
    (else
      (Utilities|FlowControl|Gate true) ; enters at Close
    )))

(event EventBeginPlay
  (bind _returnvalue (UserInterface|CreateWidget "/Game/HUDWidget.HUDWidget_C" (Game|GetPlayerController 0)))
  (UserInterface|Viewport|AddtoViewport _returnvalue 0)
  (bind _outactors (Actor|GetAllActorsOfClass "/Game/2DSideScrollerBP/Blueprints/LevelDB.LevelDB_C")))

(event EventTick
  (params (DeltaSeconds :type Float%20%28single-precision%29)))

(event EventDrawHUD
  (params (SizeX :type Integer) (SizeY :type Integer))
  (bind _returnvalue (Math|Conversions|ToFloat(Integer) SizeY))
  (bind _returnvalue_2 (Math|Conversions|ToFloat(Integer) SizeX))
  (bind _returnvalue_3 (/ _returnvalue 2.0))
  (bind _returnvalue_4 (/ _returnvalue_2 2.0))
  (bind _returnvalue_5 (+ _returnvalue_3 5e+01))
  (Utilities|FlowControl|Gate true
    (:Exit
      (if (stale EventWinLoss Win)
        (HUD|DrawText "YOU WIN!!!!!" "(R=0.000000,G=0.462077,B=0.049707,A=1.000000)" _returnvalue_4 _returnvalue_3 "/Engine/EngineFonts/Roboto.Roboto" 5.0 false)
        (HUD|DrawText "Press Enter to Move to the next Level" "(R=0.000000,G=0.463333,B=0.050678,A=1.000000)" (- _returnvalue_4 2e+02) _returnvalue_5 "/Engine/EngineFonts/Roboto.Roboto" 5.0 false)
        (Variables|/Game/2DSideScrollerBP/Blueprints/LevelDB.LevelDB_C|SetWinLoss (Utilities|Array|Get(acopy) (stale EventBeginPlay _outactors)) true)
        (else
          (HUD|DrawText "You Lose!!" "(R=0.672443,G=0.000000,B=0.000000,A=1.000000)" _returnvalue_4 _returnvalue_3 "/Engine/EngineFonts/Roboto.Roboto" 5.0 false)
          (HUD|DrawText "Press Enter to Restart" "(R=0.666666,G=0.000000,B=0.000000,A=1.000000)" (- _returnvalue_4 9e+01) _returnvalue_5 "/Engine/EngineFonts/Roboto.Roboto" 5.0 false)
          (Variables|/Game/2DSideScrollerBP/Blueprints/LevelDB.LevelDB_C|SetWinLoss (Utilities|Array|Get(acopy) (stale EventBeginPlay _outactors)) false)))
      (Variables|/Game/2DSideScrollerBP/Blueprints/LevelDB.LevelDB_C|SetCanRestart (Utilities|Array|Get(acopy) (stale EventBeginPlay _outactors)) true))))

(event EventWinLoss
  (params (Win :type Boolean)))

(fn ConstructionScript)